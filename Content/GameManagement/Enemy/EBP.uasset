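; Enemy character that endlessly chases the player and can be killed by damage.
; BeginPlay starts an AI MoveTo on the player character, which reissues itself on success or failure.
; Damage lowers clamped health, playing a random hit-react montage with a brief movement stop.
; At zero health it plays sound and a death montage, increments the player's KillCount, sometimes fires an unused downward trace, and destroys itself without delay.
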(event Custom|Chase%20Plyer
  (params (pLAYER :type Ue%204ASP%20Character%20Object%20Reference))
  (AI|AIMoveTo self "0, 0, 0" pLAYER 5.0 false
    (:OnSuccess
      _)
    (:OnFail
      _))
  (CallFunction|ChasePlyer (Variables|Default|GetAs%20Ue%204ASP%20Character)))

(event EventBeginPlay
  (bind _asue_4asp_character (Utilities|Casting|CastToUe4ASP_Character (Game|GetPlayerCharacter 0)))
  (bind _output_get (Variables|Default|SetAs%20Ue%204ASP%20Character _asue_4asp_character))
  (CallFunction|ChasePlyer _output_get))

(event Game|Damage|EventAnyDamage
  (params (Damage :type Float%20%28single-precision%29) (DamageType :type Damage%20Type%20Object%20Reference) (InstigatedBy :type Controller%20Object%20Reference) (DamageCauser :type Actor%20Object%20Reference))
  (bind _returnvalue (Transformation|GetActorLocation))
  (bind _returnvalue_2 (Transformation|GetActorLocation))
  (if (not (Variables|Default|GetIfDead))
    (bind _output_get (Variables|Default|SetHealth (Math|Float|Clamp(Float) (- (Variables|Default|GetHealth) Damage) 0.0 1e+02)))
    (if (== _output_get 0.0)
      (Audio|PlaySoundatLocation "/Game/StarterContent/Audio/Collapse01.Collapse01" _returnvalue "0, 0, 0" 1.0 1.0 0.0 0 0 0)
      (Pawn|Components|CharacterMovement|DisableMovement (Variables|Character|GetCharacterMovement))
      (Variables|Default|SetIfDead true)
      (Animation|PlayAnimMontage (Utilities|Select :Index (Math|Random|RandomInteger 3) :Option%200 "/Game/GameManagement/Animation/Death_1_Montage.Death_1_Montage" :Option%201 "/Game/GameManagement/Animation/Death_2_Montage.Death_2_Montage" :Option%202 "/Game/GameManagement/Animation/Death_3_Montage.Death_3_Montage") 1.0 "None")
      (Utilities|FlowControl|Sequence
        (:then_0
          (bind _asue_4asp_character (Utilities|Casting|CastToUe4ASP_Character (Game|GetPlayerCharacter 0)))
          (Math|Integer|IncrementInt (Variables|/Game/GameManagement/Character/Ue4ASP_Character.Ue4ASP_Character_C|GetKill%20Count _asue_4asp_character)
            (:%20%20
              (if (Math|Random|RandomBoolwithWeight 0.45)
                (Collision|LineTraceByChannel _returnvalue_2 (- _returnvalue_2 "0, 0,1500.000000") "TraceTypeQuery1" false 0 "None")))))
        (:then_1
          (Actor|DestroyActor)))
      (else
        (Audio|PlaySoundatLocation 0 _returnvalue "0, 0, 0" 1.0 1.0 0.0 0 0 0)
        (Pawn|Components|CharacterMovement|DisableMovement (Variables|Character|GetCharacterMovement))
        (Animation|PlayAnimMontage (Utilities|Select :Index (Math|Random|RandomInteger 4) :Option%200 "/Game/GameManagement/Animation/Hit_React_1_Montage.Hit_React_1_Montage" :Option%201 "/Game/GameManagement/Animation/Hit_React_2_Montage.Hit_React_2_Montage" :Option%202 "/Game/GameManagement/Animation/Hit_React_3_Montage.Hit_React_3_Montage" :Option%203 "/Game/GameManagement/Animation/Hit_React_4_Montage.Hit_React_4_Montage") 1.0 "None")
        (Utilities|FlowControl|Delay 0.2)
        (if (not (Variables|Default|GetIfDead))
          (Pawn|Components|CharacterMovement|SetMovementMode (Variables|Character|GetCharacterMovement) "MOVE_Walking" 0))))))

(fn ConstructionScript)