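; BP_ENEMY_SPAWNER is an actor that repeatedly spawns waves of enemies at its own transform.
; On BeginPlay it calls a custom EnemySpawner event with the configured enemy class and count.
; That event spawns the batch in a loop, waits for the Duration delay, then calls itself again, so waves continue with no stop condition in the graph.
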(event Custom|Enemy%20Spawner
  (params (Enemy :type Actor%20Class%20Reference) (SpawnTransform :type Transform) (No%20Enemy :type Integer))
  (for _index (range 0 (- No%20Enemy 1))
    (Game|SpawnActorfromClass Enemy SpawnTransform "Undefined" 0 0))
  (Utilities|FlowControl|Delay (Variables|Default|GetDuration))
  (CallFunction|EnemySpawner (Variables|Default|GetEnemy) (Transformation|GetActorTransform) (Variables|Default|GetNo%20Enemy)))

(event EventBeginPlay
  (CallFunction|EnemySpawner (Variables|Default|GetEnemy) (Transformation|GetActorTransform) (Variables|Default|GetNo%20Enemy)))

(fn ConstructionScript)